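; BP_ExamineObject is an examinable world object whose static mesh is set from ObjectModel in the construction script.
; ExamineObject toggles the examining state, printing a message and returning ObjectModel only when examination starts.
; Instead of hiding the actor, it saves the location and teleports it to the world origin, then teleports it back when put back.
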(event `Move Object Away`
  (set `self.ObjectLocation` (`self.K2_GetActorLocation`))
  (`self.K2_SetActorLocation` (0.0 0.0 0.0) false true))

(event `Move Object Back`
  (`self.K2_SetActorLocation` (`self.ObjectLocation`) false true))

(fn `ExamineObject`
  (returns (ObjectModel :type "StaticMesh Object Reference"))
  (if (`self.isExamining`)
    (set `self.isExamining` false)
    (`KismetSystemLibrary.PrintString` "Object Put Back")
    (`self.Move Object Back`)
    (else
      (set `self.isExamining` true)
      (`KismetSystemLibrary.PrintString` "Object Examined")
      (`self.Move Object Away`)
      (return (`self.ObjectModel`)))))

(fn `UserConstructionScript`
  (`StaticMeshComponent.SetStaticMesh` (`self.StaticMesh`) (`self.ObjectModel`)))